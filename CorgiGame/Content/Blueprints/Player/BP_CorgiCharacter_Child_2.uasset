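; Child corgi player character Blueprint that adds a bark action, with a stronger interacting bark when the Fey flag is set.
; With Fey set, barking plays a sound, activates the big-bark emitter and line traces ahead of the mesh, correcting its yaw by 90 degrees.
; A hit stores the impact point and sends an interact message to that actor.
; Without Fey, barking only plays an alternate sound.
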(event EventBeginPlay
  (|CallParentFunction) ; This node is disabled and will not be called.\nDrag off pins to build functionality.
)

(event Collision|EventActorBeginOverlap
  (params (OtherActor :type Actor%20Object%20Reference))
  (|CallParentFunction OtherActor) ; This node is disabled and will not be called.\nDrag off pins to build functionality.
)

(event EventTick
  (params (DeltaSeconds :type Float%20%28single-precision%29))
  (|CallParentFunction DeltaSeconds) ; This node is disabled and will not be called.\nDrag off pins to build functionality.
)

(event Input|ActionEvents|InputActionBark
  (params (Key :type Key%20Structure :default "None"))
  (bind _mesh (Variables|Character|GetMesh))
  (bind _returnvalue (Transformation|GetWorldLocation _mesh))
  (bind _returnvalue_2 (Transformation|GetWorldRotation _mesh))
  (:Pressed
    (if (Variables|Default|GetFey?)
      (Audio|PlaySound2D "/Game/Audio/Dog/Barks/AlertBark2.AlertBark2" 1.0 1.0 0.0 0 0)
      (Components|Activation|Activate (Variables|Default|GetNS_BigBarkEmitter) true)
      (bind (_outhit _returnvalue_3) (Collision|LineTraceByChannel (+ _returnvalue "0,0.000000,50.000000") (+ (+ _returnvalue (* (Math|Vector|GetForwardVector (Math|Rotator|MakeRotator (.roll _returnvalue_2) (.pitch _returnvalue_2) (+ (.yaw _returnvalue_2) 9e+01))) 5e+02)) "0,0.000000,50.000000") "TraceTypeQuery1" false 0 "None"))
      (if _returnvalue_3
        (Variables|Default|SetHitLocation (.ImpactPoint (Collision|BreakHitResult _outhit)))
        (Class|BPIBarkInterface|Interact(Message) (.HitActor (Collision|BreakHitResult _outhit))))
      (else
        (Audio|PlaySound2D "/Game/Audio/Dog/Barks/AlertBark3.AlertBark3" 1.0 1.0 0.0 0 0)))))

(fn ConstructionScript
  (|CallParentFunction))