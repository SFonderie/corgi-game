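; BP_NPC is an AI-controlled character that can act as a follower of a target, optionally the player.
; On BeginPlay it runs its Behavior Tree on the AI controller and, if PlayerIsTarget is set, takes the player character as Target.
; For followers, Tick calls FollowTarget, which only switches max walk speed: slow inside FollowRadius of the target, fast otherwise.
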(event EventBeginPlay
  (bind _asaicontroller (Utilities|Casting|CastToAIController (Pawn|GetController)))
  (AI|RunBehaviorTree _asaicontroller (Variables|Default|GetBehavior%20Tree))
  (if (Variables|Default|GetPlayerIsTarget)
    (Variables|Default|SetTarget (Game|GetPlayerCharacter 0))))

(event Collision|EventActorBeginOverlap
  (params (OtherActor :type Actor%20Object%20Reference)))

(event EventTick
  (params (DeltaSeconds :type Float%20%28single-precision%29))
  (if (Variables|Default|GetIsFollower)
    (CallFunction|FollowTarget)))

(fn ConstructionScript)

(fn FollowTarget
  (Variables|/Script/Engine.CharacterMovementComponent|SetMaxWalkSpeed (Variables|Character|GetCharacterMovement) (Math|Float|SelectFloat 1.5e+02 4.5e+02 (> (Variables|Default|GetFollow%20Radius) (Transformation|GetDistanceTo (Variables|Default|GetTarget))))))