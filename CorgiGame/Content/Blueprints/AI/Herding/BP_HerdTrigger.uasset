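; BP_HerdTrigger is a trigger actor that herds its Target NPC into a contained area when overlapped by an actor of the Target's class.
; The overlap switches Target to a stationary behavior tree, then AI-moves it to a random navigable point around OriginPoint, using WanderRadius and the BP_HerdFilter navigation filter.
; Target then runs the contained behavior tree, whether the move succeeds or fails.
; The class match acts on the stored Target, not the overlapping actor.
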(event EventBeginPlay)

(event Collision|EventActorBeginOverlap
  (params (OtherActor :type Actor%20Object%20Reference))
  (bind _target (Variables|Default|GetTarget))
  (bind _returnvalue (AI|GetAIController _target))
  (if (== (Utilities|GetClass OtherActor) (Utilities|GetClass (Variables|Default|GetTarget)))
    (bind _output_get (Variables|/Game/Blueprints/AI/BP_NPC.BP_NPC_C|SetBehavior%20Tree _target "/Game/Blueprints/AI/Trees/BT_NPC_Stationary.BT_NPC_Stationary"))
    (AI|RunBehaviorTree _returnvalue _output_get)
    (bind _output_get_2 (Variables|Default|SetHerdOrigin (Transformation|GetActorLocation (Variables|Default|GetOriginPoint))))
    (bind _randomlocation (Class|NavigationSystemV1|GetRandomLocationinNavigableRadius _output_get_2 (Variables|Default|GetWanderRadius) 0 "/Game/Blueprints/AI/Herding/BP_HerdFilter.BP_HerdFilter_C"))
    (AI|AIMoveTo _target _randomlocation 0 5.0 false
      (:OnSuccess
        _)
      (:OnFail
        _))
    (bind _output_get_3 (Variables|/Game/Blueprints/AI/BP_NPC.BP_NPC_C|SetBehavior%20Tree _target "/Game/Blueprints/AI/Trees/BT_NPC_Contained.BT_NPC_Contained"))
    (AI|RunBehaviorTree _returnvalue _output_get_3)
    (else
      (Development|PrintString "Wrong Target"))))

(event EventTick
  (params (DeltaSeconds :type Float%20%28single-precision%29)))

(fn ConstructionScript)