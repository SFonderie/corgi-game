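; BP_HerdTrigger is an overlap trigger that herds a preset Target NPC into a navigable area around an OriginPoint actor.
; When an actor of Target's class overlaps, it sets Target's BehaviorTree to stationary and AI-moves Target to a random point within WanderRadius, filtered by BP_HerdFilter.
; Success or failure of the move both switch Target to the contained tree; other classes only print "Wrong Target".
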(event EventBeginPlay)

(event Collision|EventActorBeginOverlap
  (params (OtherActor :type Actor%20Object%20Reference))
  (bind _target (Variables|Default|GetTarget))
  (if (== (Utilities|GetClass OtherActor) (Utilities|GetClass (Variables|Default|GetTarget)))
    (Variables|/Game/Blueprints/AI/BP_NPC.BP_NPC_C|SetBehavior%20Tree _target "/Game/Blueprints/AI/Trees/BT_NPC_Stationary.BT_NPC_Stationary")
    (bind _output_get (Variables|Default|SetHerdOrigin (Transformation|GetActorLocation (Variables|Default|GetOriginPoint))))
    (bind _randomlocation (Class|NavigationSystemV1|GetRandomLocationinNavigableRadius _output_get (Variables|Default|GetWanderRadius) 0 "/Game/Blueprints/AI/BP_HerdFilter.BP_HerdFilter_C"))
    (AI|AIMoveTo _target _randomlocation 0 5.0 false
      (:OnSuccess
        _)
      (:OnFail
        _))
    (Variables|/Game/Blueprints/AI/BP_NPC.BP_NPC_C|SetBehavior%20Tree _target "/Game/Blueprints/AI/Trees/BT_NPC_Contained.BT_NPC_Contained")
    (else
      (Development|PrintString "Wrong Target"))))

(event EventTick
  (params (DeltaSeconds :type Float%20%28single-precision%29)))

(fn ConstructionScript)