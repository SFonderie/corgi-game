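; BP_BarkableBox is an interactable box that the corgi player can shatter, only while the character's Fey flag is set.
; On Interact it casts the player to BP_CorgiCharacter_Child_2, destroys the intact static mesh and reveals a physics-simulated Destructible.
; It applies heavy damage at the character's HitLocation, with an impulse derived from the player-to-box direction plus the box's location, then destroys itself after a short delay.
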(event EventInteract
  (bind _returnvalue (Transformation|GetActorLocation))
  (bind _asbp_corgi_character_child_2 (Utilities|Casting|CastToBP_CorgiCharacter_Child_2 (Game|GetPlayerCharacter 0)))
  (if (Variables|/Game/Blueprints/Player/BP_CorgiCharacter_Child_2.BP_CorgiCharacter_Child_2_C|GetFey? _asbp_corgi_character_child_2)
    (Components|DestroyComponent (Variables|Default|GetStaticMesh))
    (Development|SetHiddeninGame (Variables|Default|GetDestructible) false false)
    (Physics|SetSimulatePhysics (Variables|Default|GetDestructible) true)
    (Class|DestructibleComponent|ApplyDamage (Variables|Default|GetDestructible) 5e+03 (Variables|/Game/Blueprints/Player/BP_CorgiCharacter_Child_2.BP_CorgiCharacter_Child_2_C|GetHitLocation _asbp_corgi_character_child_2) (+ (* (Math|Vector|GetUnitDirection(Vector) (Transformation|GetActorLocation _asbp_corgi_character_child_2) _returnvalue) 2e+02) _returnvalue) 5e+03)
    (Utilities|FlowControl|Delay 2.5)
    (Actor|DestroyActor)))

(fn ConstructionScript)