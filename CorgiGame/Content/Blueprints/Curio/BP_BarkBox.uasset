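; BP_BarkBox is a curio box that gets physically shoved when it receives one specific interaction type.
; On that interaction, BoxMesh gets a mass-independent velocity-change impulse along a normalized difference of actor locations.
; Impulse strength is Force divided by the square root of that distance, an inverse square root falloff despite the "Inverse Square" comment.
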(event EventOnInteraction
  (params (PlayerCharacter :type BP%20Corgi%20Character%20Object%20Reference) (Interaction :type BPE_Interaction%20Enum :default "NewEnumerator8"))
  (bind _returnvalue (Transformation|GetActorLocation))
  (bind _self self)
  (bind _returnvalue_2 (Transformation|GetActorLocation _self))
  (bind _returnvalue_3 (- _returnvalue_2 _returnvalue))
  (bind _returnvalue_4 (Math|Vector|VectorLength _returnvalue_3))
  (if (Utilities|Enum|Equal(Enum) Interaction "NewEnumerator2")
    (Physics|AddImpulse (Variables|Default|GetBoxMesh) (* (/ _returnvalue_3 _returnvalue_4) (/ (Variables|Default|GetForce) (Math|Float|Sqrt _returnvalue_4))) "None" true)))

(fn ConstructionScript)