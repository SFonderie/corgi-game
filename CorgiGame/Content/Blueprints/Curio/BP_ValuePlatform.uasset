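; BP_ValuePlatform is a platform whose position between two control points is driven by a value passed to SetValue.
; SetValue scales the value by ValueFactor and folds it with modulo and floor into a triangle wave, so rising values ping-pong the mesh between the points.
; GetPoints resolves each point as absolute or as an offset from the actor's location.
; The mesh moves without sweep, and the actor runs no Tick logic.
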(event EventBeginPlay)

(event Collision|EventActorBeginOverlap
  (params (OtherActor :type Actor%20Object%20Reference)))

(event EventTick
  (params (DeltaSeconds :type Float%20%28single-precision%29)))

(fn ConstructionScript)

(fn SetValue
  (params (Value :type Float%20%28single-precision%29))
  (bind (_point_a _point_b) (CallFunction|GetPoints))
  (bind _value_factor (Variables|Settings|GetValue%20Factor))
  (bind _returnvalue (* Value _value_factor))
  (bind _returnvalue_2 (Math|Float|%(Float) _returnvalue 2.0))
  (bind _returnvalue_3 (Math|Float|Floor _returnvalue_2))
  (Transformation|SetWorldLocation (Variables|Default|GetPlatform%20Mesh) (Math|Vector|Lerp(Vector) _point_a _point_b (+ (Math|Conversions|ToFloat(Integer) _returnvalue_3) (* (+ (* _returnvalue_3 -2) 1) (Math|Float|%(Float) _returnvalue 1.0)))) false false))

(fn GetPoints
  (bind _returnvalue (Transformation|GetActorLocation))
  (bind _control_point_a (Variables|Settings|GetControl%20Point%20A))
  (bind _control_point_b (Variables|Settings|GetControl%20Point%20B))
  (return (Math|Vector|SelectVector (+ _returnvalue (.positioncontrolpoint _control_point_a)) (.positioncontrolpoint _control_point_a) (.bpositionisrelative _control_point_a)) (Math|Vector|SelectVector (+ _returnvalue (.positioncontrolpoint _control_point_b)) (.positioncontrolpoint _control_point_b) (.bpositionisrelative _control_point_b))))