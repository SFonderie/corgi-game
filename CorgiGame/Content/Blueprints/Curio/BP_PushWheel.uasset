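; BP_PushWheel is a physical wheel that tracks how many turns it has made and reports that count to a listener.
; Each tick it takes the yaw change of WheelCore since the last stored rotation, converts it to turns and adds it to Rotations.
; The per-tick change is clamped to a small range to prevent resets at yaw wraparound.
; The running total is passed to Listener through SetValue whenever the listener is valid.
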(event EventTick
  (params (DeltaSeconds :type Float%20%28single-precision%29))
  (bind _wheelcore (Variables|Default|GetWheelCore))
  (bind _returnvalue (Transformation|GetWorldRotation _wheelcore))
  ;[1 1 1] Update Rotations
  (Variables|State|SetRotations (+ (Variables|State|GetRotations) (Math|Float|Clamp(Float) (/ (- (.Yaw (Math|Rotator|BreakRotator _returnvalue)) (.Yaw (Math|Rotator|BreakRotator (Variables|State|GetTrackRotation)))) 3.6e+02) -0.01 0.01)))
  (Variables|State|SetTrackRotation _returnvalue)
  (Utilities|IsValid (Variables|Default|GetListener)
    (:Is%20Valid
      (Default|SetValue (Variables|Default|GetListener) (Variables|State|GetRotations)))))

(fn ConstructionScript)