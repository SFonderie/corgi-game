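; BP_Slippers is a grabbable slippers prop that either corgi character can pick up and drop.
; OnGrab casts the invoker to BP_CorgiCharacter or BP_CorgiCharacterPerspective, setting GrabbedItem on the latter.
; A separate FlipFlop per branch alternates between attaching with the cube's collision and physics off, and detaching with both restored.
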(event EventOnGrab
  (params (Invoker :type Character%20Object%20Reference))
  (bind _cube (Variables|Default|GetCube))
  (bind _cube_2 (Variables|Default|GetCube))
  (bind _asbp_corgi_character (Utilities|Casting|CastToBP_CorgiCharacter Invoker)
    (:then
      (Utilities|FlowControl|FlipFlop
        (:A
          (Transformation|AttachActorToActor _asbp_corgi_character "None" "KeepWorld" "KeepRelative" "KeepRelative" true)
          (Collision|SetCollisionEnabled _cube_2 "NoCollision")
          (Physics|SetSimulatePhysics _cube_2 false))
        (:B
          (Transformation|DetachFromActor "KeepWorld" "KeepRelative" "KeepRelative")
          (Collision|SetCollisionEnabled _cube_2 "QueryAndPhysics")
          (Physics|SetSimulatePhysics _cube_2 true))))
    (:CastFailed
      (bind _asbp_corgi_character_perspective (Utilities|Casting|CastToBP_CorgiCharacterPerspective Invoker))
      (Variables|/Game/Blueprints/Player/BP_CorgiCharacterPerspective.BP_CorgiCharacterPerspective_C|SetGrabbedItem _asbp_corgi_character_perspective self)
      (Utilities|FlowControl|FlipFlop
        (:A
          (Transformation|AttachActorToActor _asbp_corgi_character_perspective "None" "KeepWorld" "KeepRelative" "KeepRelative" true)
          (Collision|SetCollisionEnabled _cube "NoCollision")
          (Physics|SetSimulatePhysics _cube false))
        (:B
          (Transformation|DetachFromActor "KeepWorld" "KeepRelative" "KeepRelative")
          (Collision|SetCollisionEnabled _cube "QueryAndPhysics")
          (Physics|SetSimulatePhysics _cube true))))))

(fn ConstructionScript)