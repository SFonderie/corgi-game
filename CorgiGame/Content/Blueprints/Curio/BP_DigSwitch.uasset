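; BP_DigSwitch is a curio actor that starts buried and switches to an unburied mesh when it receives a specific interaction.
; BeginPlay sets the buried flag and caches the actor's location.
; OnInteraction checks the interaction enum, then swaps the static mesh, clears the flag and moves the actor to the cached location.
; An offset move by SwapOffset is present but disconnected, so it never runs.
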(event EventOnInteraction
  (params (PlayerCharacter :type BP%20Corgi%20Character%20Object%20Reference) (Interaction :type BPE_Interaction%20Enum :default "NewEnumerator8"))
  (if (Utilities|Enum|Equal(Enum) Interaction "NewEnumerator1")
    (Components|StaticMesh|SetStaticMesh (Variables|Debug|GetStaticMeshComponent) (Variables|Default|GetNew%20Mesh))
    (Variables|Default|SetIs%20Burried false)
    (Transformation|SetActorLocation (Variables|Default|GetActorLoc) false false)))

(event EventBeginPlay
  (Variables|Default|SetIs%20Burried true)
  (Variables|Default|SetActorLoc (Transformation|GetActorLocation)))

(fn ConstructionScript)