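; Actor that repeatedly fires BP_Projectile toward the first player character.
; Tick feeds a Delay of FireDelay, which acts as a repeating fire timer.
; Each shot spawns half-scale at a small world-X offset from the spawner, rotated to face the player's current location.
; The spawner copies its speed, impact, arc impulse and fire delay settings onto the projectile, then calls Spawned on it.
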(event EventBeginPlay)

(event Collision|EventActorBeginOverlap
  (params (OtherActor :type Actor%20Object%20Reference)))

(event EventTick
  (params (DeltaSeconds :type Float%20%28single-precision%29))
  (bind _returnvalue (Transformation|GetActorLocation))
  (bind _returnvalue_2 (+ _returnvalue "15.000000, 0,0.000000"))
  (Utilities|FlowControl|Delay (Variables|Default|GetFireDelay))
  (bind _returnvalue_3 (Game|SpawnActorfromClass "/Game/Blueprints/Curio/BP_Projectile.BP_Projectile_C" (Math|Transform|MakeTransform _returnvalue_2 (Math|Rotator|FindLookatRotation _returnvalue_2 (Transformation|GetActorLocation (Game|GetPlayerCharacter 0))) "0.500000,0.500000,0.500000") "AdjustIfPossibleButAlwaysSpawn" 0 0))
  (Variables|/Game/Blueprints/Curio/BP_Projectile.BP_Projectile_C|SetSpeed _returnvalue_3 (Variables|Default|GetSpeed))
  (Variables|/Game/Blueprints/Curio/BP_Projectile.BP_Projectile_C|SetImpact _returnvalue_3 (Variables|Default|GetImpact))
  (Variables|/Game/Blueprints/Curio/BP_Projectile.BP_Projectile_C|SetArcImpulse _returnvalue_3 (Variables|Default|GetArcImpulse))
  (Variables|/Game/Blueprints/Curio/BP_Projectile.BP_Projectile_C|SetFireDelay _returnvalue_3 (Variables|Default|GetFireDelay))
  (Default|Spawned _returnvalue_3))

(fn ConstructionScript)