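; BP_DialogueBox is an actor that shows multi-line dialogue through a BP_DialogueUI widget.
; Beginning an overlap creates the widget and adds it to the viewport, and ending it removes the widget.
; A matching interaction passes the DialogueText array to the widget, reveals its text and box, then advances TextRow or removes it at the last row.
; A DoOnce, reset after each step, gates the interaction.
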(event Custom|Dialogue%20Reset
  (bind _dialogueui (Variables|Default|GetDialogueUI))
  (bind _dialoguetext (Variables|Default|GetDialogueText))
  (bind _dialogueui_2 (Variables|Default|GetDialogueUI))
  (Utilities|FlowControl|DoOnce false) ; enters at Reset
)

(event EventOnInteraction
  (params (PlayerCharacter :type BP%20Corgi%20Character%20Object%20Reference) (Interaction :type BPE_Interaction%20Enum :default "NewEnumerator8"))
  (bind _dialogueui (Variables|Default|GetDialogueUI))
  (bind _dialoguetext (Variables|Default|GetDialogueText))
  (bind _dialogueui_2 (Variables|Default|GetDialogueUI))
  (if (Utilities|Enum|Equal(Enum) Interaction "NewEnumerator2")
    (Utilities|FlowControl|DoOnce false
      (:Completed
        (Variables|/Game/Blueprints/Player/BP_DialogueUI.BP_DialogueUI_C|SetText _dialogueui _dialoguetext)
        (Widget|SetVisibility (Variables|/Game/Blueprints/Player/BP_DialogueUI.BP_DialogueUI_C|GetDialogueText _dialogueui) "Visible")
        (if (> (+ (Variables|/Game/Blueprints/Player/BP_DialogueUI.BP_DialogueUI_C|GetTextRow _dialogueui) 1) (- (Utilities|Array|Length _dialoguetext) 1))
          (Widget|RemovefromParent _dialogueui_2)
          (else
            (Variables|/Game/Blueprints/Player/BP_DialogueUI.BP_DialogueUI_C|SetTextRow _dialogueui_2 (+ (Variables|/Game/Blueprints/Player/BP_DialogueUI.BP_DialogueUI_C|GetTextRow _dialogueui) 1))))
        (CallFunction|DialogueReset)))))

(event Collision|EventActorEndOverlap
  (params (OtherActor :type Actor%20Object%20Reference))
  (bind _dialogueui (Variables|Default|GetDialogueUI))
  ;[1 1 1] Find a better way than a separate overlap check here if possible, otherwise, oh well.
  (Utilities|IsValid _dialogueui
    (:Is%20Valid
      (Widget|RemovefromParent _dialogueui))))

(event Collision|EventActorBeginOverlap
  (params (OtherActor :type Actor%20Object%20Reference))
  ;[1 1 1] Find a better way than a separate overlap check here if possible, otherwise, oh well.
  (bind _returnvalue (UserInterface|CreateWidget "/Game/Blueprints/Player/BP_DialogueUI.BP_DialogueUI_C"))
  (bind _output_get (Variables|Default|SetDialogueUI _returnvalue))
  (UserInterface|Viewport|AddtoViewport _output_get 0))

(fn ConstructionScript)