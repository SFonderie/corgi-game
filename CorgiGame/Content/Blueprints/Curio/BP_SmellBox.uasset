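; BP_SmellBox is a trigger box actor tied to a smell-o-vision highlight effect in post-processing.
; Character overlap with the box sets a flag, named IsSpin despite no rotation logic, and end overlap clears it.
; While the flag is set, Tick casts the scene post-process volume and sets post-process settings members on the highlight struct every frame.
; Nothing here reverts those settings on exit.
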(event OnComponentBeginOverlap(BoxTrigger)
  (params (OverlappedComponent :type Primitive%20Component%20Object%20Reference) (OtherActor :type Actor%20Object%20Reference) (OtherComp :type Primitive%20Component%20Object%20Reference) (OtherBodyIndex :type Integer) (bFromSweep :type Boolean) (SweepResult :type Hit%20Result%20Structure%20%28by%20ref%29))
  (Utilities|Casting|CastToCharacter OtherActor)
  (Variables|Default|SetIsSpin true))

(event OnComponentEndOverlap(BoxTrigger)
  (params (OverlappedComponent :type Primitive%20Component%20Object%20Reference) (OtherActor :type Actor%20Object%20Reference) (OtherComp :type Primitive%20Component%20Object%20Reference) (OtherBodyIndex :type Integer))
  (Utilities|Casting|CastToCharacter OtherActor)
  (Variables|Default|SetIsSpin false))

(event EventBeginPlay)

(event Collision|EventActorBeginOverlap
  (params (OtherActor :type Actor%20Object%20Reference)))

(event EventTick
  (params (DeltaSeconds :type Float%20%28single-precision%29))
  (if (Variables|Default|GetIsSpin) ; Do spin?
    (Utilities|Casting|CastToPostProcessVolume (Variables|Default|GetScenePostProcessVolume))
    (Utilities|Struct|SetmembersinPostProcessSettings (Variables|Default|GetSmellOVisionHighlight) "(Array=)")))

(fn ConstructionScript)