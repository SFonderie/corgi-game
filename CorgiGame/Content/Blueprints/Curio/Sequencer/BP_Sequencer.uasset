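; BP_Sequencer is a Curio Blueprint with event hooks for nudge, bark, dig, flip, grab, player enter and character enter interactions.
; Each event tests a bit of InteractionMask to gate its response, but every branch and the construction script are empty.
; Both enter events test the same bit as grab instead of separate flags of their own.
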(event EventOnBark
  (params (Invoker :type Character%20Object%20Reference))
  (if (> (Class|KismetMathLibrary|AndIntInt (Variables|Settings|GetInteractionMask) (|BitmaskLiteral 2)) 0)
    _))

(event EventOnDig
  (params (Invoker :type Character%20Object%20Reference))
  (if (> (Class|KismetMathLibrary|AndIntInt (Variables|Settings|GetInteractionMask) (|BitmaskLiteral 4)) 0)
    _))

(event EventOnFlip
  (params (Invoker :type Character%20Object%20Reference))
  (if (> (Class|KismetMathLibrary|AndIntInt (Variables|Settings|GetInteractionMask) (|BitmaskLiteral 8)) 0)
    _))

(event EventOnNudge
  (params (Invoker :type Character%20Object%20Reference))
  (if (> (Class|KismetMathLibrary|AndIntInt (Variables|Settings|GetInteractionMask) (|BitmaskLiteral 1)) 0)
    _))

(event EventOnGrab
  (params (Invoker :type Character%20Object%20Reference))
  (if (> (Class|KismetMathLibrary|AndIntInt (Variables|Settings|GetInteractionMask) (|BitmaskLiteral 16)) 0)
    _))

(event EventOnPlayerEnter
  (params (Player :type Character%20Object%20Reference))
  (if (> (Class|KismetMathLibrary|AndIntInt (Variables|Settings|GetInteractionMask) (|BitmaskLiteral 16)) 0)
    _))

(event EventOnCharacterEnter
  (params (Character :type Character%20Object%20Reference))
  (if (> (Class|KismetMathLibrary|AndIntInt (Variables|Settings|GetInteractionMask) (|BitmaskLiteral 16)) 0)
    _))

(fn ConstructionScript)