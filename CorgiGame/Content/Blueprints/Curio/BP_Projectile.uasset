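; BP_Projectile is a physics-driven projectile that knocks the player's corgi character on contact.
; On BeginPlay it launches its Sphere with a fixed impulse, mostly along world Y with slight lift.
; On actor overlap, if the other actor's class matches the player's BP_CorgiCharacter, it applies an impulse to that character's movement component, scaled from the Sphere's current velocity by Speed.
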(event EventBeginPlay
  (Physics|AddImpulse (Variables|Default|GetSphere) "0,100.000000,5.000000" "None" false))

(event EventTick
  (params (DeltaSeconds :type Float%20%28single-precision%29)))

(event Collision|EventActorBeginOverlap
  (params (OtherActor :type Actor%20Object%20Reference))
  (bind _asbp_corgi_character (Utilities|Casting|CastToBP_CorgiCharacter (Game|GetPlayerCharacter 0)))
  (if (== (Utilities|GetClass _asbp_corgi_character) (Utilities|GetClass OtherActor))
    (Physics|AddImpulse (Variables|/Script/Engine.Character|GetCharacterMovement _asbp_corgi_character) (* (Transformation|GetComponentVelocity (Variables|Default|GetSphere)) (* (Variables|Default|GetSpeed) 1.0)) false)))

(fn ConstructionScript)