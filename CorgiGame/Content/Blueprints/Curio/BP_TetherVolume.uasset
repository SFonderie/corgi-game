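; BP_TetherVolume is an overlap volume that suspends a character's movement input and pushes against its horizontal motion on entry.
; On begin overlap it ignores controller move input and applies a mass-dependent CharacterMovement impulse built from last update velocity, with X and Y reversed and doubled and Z unchanged.
; On end overlap it releases the move-input ignore; non-Character actors are skipped.
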(event Collision|EventActorEndOverlap
  (params (OtherActor :type Actor%20Object%20Reference))
  (bind _ascharacter (Utilities|Casting|CastToCharacter OtherActor))
  (Input|SetIgnoreMoveInput (Pawn|GetController _ascharacter) false))

(event Collision|EventActorBeginOverlap
  (params (OtherActor :type Actor%20Object%20Reference))
  (bind _ascharacter (Utilities|Casting|CastToCharacter OtherActor))
  (Input|SetIgnoreMoveInput (Pawn|GetController _ascharacter) true)
  (Physics|AddImpulse (Variables|/Script/Engine.Character|GetCharacterMovement _ascharacter) (Math|Vector|MakeVector (* (.X (Math|Vector|BreakVector (Pawn|Components|CharacterMovement|GetLastUpdateVelocity (Variables|/Script/Engine.Character|GetCharacterMovement _ascharacter)))) -2.0) (* (.Y (Math|Vector|BreakVector (Pawn|Components|CharacterMovement|GetLastUpdateVelocity (Variables|/Script/Engine.Character|GetCharacterMovement _ascharacter)))) -2.0) (.Z (Math|Vector|BreakVector (Pawn|Components|CharacterMovement|GetLastUpdateVelocity (Variables|/Script/Engine.Character|GetCharacterMovement _ascharacter))))) false))

(fn ConstructionScript)