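; Level trigger box that notifies an array of listeners when characters enter or leave it.
; Actor begin and end overlap events ignore anything that is not a Character, then loop through every entry in Listeners.
; Player-controlled characters fire OnPlayerEnter or OnPlayerExit, while all others fire OnCharacterEnter or OnCharacterExit, each passing the character along.
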(event Collision|EventActorBeginOverlap
  (params (OtherActor :type Actor%20Object%20Reference))
  (bind _ascharacter (Utilities|Casting|CastToCharacter OtherActor)) ; Only deploy if the actor is a\nhumanoid character pawn.
  (for _array_element (Variables|Default|GetListeners) ; Loop through the listeners.
    (if (Pawn|IsPlayerControlled _ascharacter) ; Switch events depending\non the player controller.
      (Default|OnPlayerEnter _array_element _ascharacter)
      (else
        (Default|OnCharacterEnter _array_element _ascharacter)))))

(event Collision|EventActorEndOverlap
  (params (OtherActor :type Actor%20Object%20Reference))
  (bind _ascharacter (Utilities|Casting|CastToCharacter OtherActor)) ; Only deploy if the actor is a\nhumanoid character pawn.
  (for _array_element (Variables|Default|GetListeners) ; Loop through the listeners.
    (if (Pawn|IsPlayerControlled _ascharacter) ; Switch events depending\non the player controller.
      (Default|OnPlayerExit _array_element _ascharacter)
      (else
        (Default|OnCharacterExit _array_element _ascharacter)))))

(fn ConstructionScript)