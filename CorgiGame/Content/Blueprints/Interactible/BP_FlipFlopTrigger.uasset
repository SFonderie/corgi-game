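; Interactible trigger that teleports its invoker to a paired Mirror trigger, keeping their offset from the trigger.
; On BeginPlay it links itself back to its Mirror if that one has no valid partner.
; OnFlip plays the LS_FlipFade level sequence and teleports after a hard-coded delay.
; A CanTeleport flag blocks repeat flips until a second delay ends and the sequence actor is destroyed.
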(event EventOnFlip
  (params (Invoker :type Character%20Object%20Reference))
  (if (Variables|Default|GetCanTeleport) ; Ensure that button spam\ncannot break the flip.
    (Variables|Default|SetCanTeleport false)
    (bind (_outactor _returnvalue) (Sequencer|Player|CreateLevelSequencePlayer "/Game/Blueprints/Interactible/LS_FlipFade.LS_FlipFade")) ; Create a new level sequence player for the\nfade sequence and plop it... somewhere.
    (Sequencer|Player|Play _returnvalue :!class /Script/MovieScene.MovieSceneSequencePlayer) ; Actually play the level sequence.
    (Utilities|FlowControl|Delay 1.0) ; Hard-coded delay.
    (Transformation|Teleport Invoker
      (:next
        (Utilities|FlowControl|Delay 1.0) ; Hard-coded delay.
        (Actor|DestroyActor _outactor)
        (Variables|Default|SetCanTeleport true)))))

(event EventBeginPlay
  (Utilities|IsValid (Variables|Default|GetMirror)
    (:Is%20Valid
      (Utilities|IsValid (Variables|BP_FlipFlopTrigger_C|GetMirror (Variables|Default|GetMirror)) ; If we're connected to something\nand it's not connected to anything,\nconnect it to ourselves.
        (:Is%20Not%20Valid
          (Variables|BP_FlipFlopTrigger_C|SetMirror (Variables|Default|GetMirror) self))))))

(fn ConstructionScript)