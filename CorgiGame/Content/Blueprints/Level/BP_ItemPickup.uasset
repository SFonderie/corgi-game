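; Pickup item that a player character can grab, carry, drop or deliver to a target.
; On a matching interaction while active, it registers as ItemGrabbed, disables mesh physics and collision, and attaches to the player.
; Drop and deliver act only on the held item: drop calls detach on the player character and restores physics with physics-only collision.
; Delivery attaches it to a target socket and deactivates it against re-grabbing.
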(event Custom|On%20Player%20Drop
  (params (PlayerCharacter :type BP%20Corgi%20Character%20Object%20Reference))
  (Utilities|IsValid (Variables|/Game/Blueprints/Player/BP_CorgiCharacter.BP_CorgiCharacter_C|GetItemGrabbed PlayerCharacter) ; Only attempt a drop if the player\nis actually holding something...
    (:Is%20Valid
      (if (== self (Variables|/Game/Blueprints/Player/BP_CorgiCharacter.BP_CorgiCharacter_C|GetItemGrabbed PlayerCharacter)) ; And that something is actually\nourselves. We don't want to\ndrop someone else!
        (Variables|/Game/Blueprints/Player/BP_CorgiCharacter.BP_CorgiCharacter_C|SetItemGrabbed PlayerCharacter 0) ; Clear the reference.
        (Transformation|DetachFromActor PlayerCharacter "KeepWorld" "KeepRelative" "KeepRelative") ; Remove ourselves from the player.
        (Collision|SetCollisionEnabled (Variables|Default|GetItemMesh) "PhysicsOnly") ; Turn on item mesh collision.
        (Physics|SetSimulatePhysics (Variables|Default|GetItemMesh) true) ; Turn on item mesh physics.
        (Development|PrintString "Goodbye")))))

(event Custom|On%20Player%20Deliver
  (params (PlayerCharacter :type BP%20Corgi%20Character%20Object%20Reference) (DeliverTarget :type Actor%20Object%20Reference) (DeliverSocket :type Name))
  (Utilities|IsValid (Variables|/Game/Blueprints/Player/BP_CorgiCharacter.BP_CorgiCharacter_C|GetItemGrabbed PlayerCharacter) ; Only attempt delivery if the player\nis actually holding something...
    (:Is%20Valid
      (if (== self (Variables|/Game/Blueprints/Player/BP_CorgiCharacter.BP_CorgiCharacter_C|GetItemGrabbed PlayerCharacter)) ; And that something is actually\nourselves. We don't want to\ndeliver someone else!
        (Variables|/Game/Blueprints/Player/BP_CorgiCharacter.BP_CorgiCharacter_C|SetItemGrabbed PlayerCharacter 0) ; Clear the reference.
        (Transformation|AttachActorToActor DeliverTarget DeliverSocket "KeepWorld" "KeepRelative" "KeepRelative" false) ; Attach ourselves to the target.
        (Variables|State|SetIsActive false) ; Prevents the object from\nbeing grabbed again.
        (Development|PrintString "Farewell")))))

(event EventOnPlayerInteract
  (params (PlayerCharacter :type BP%20Corgi%20Character%20Object%20Reference) (Interaction :type BPE_Interaction%20Enum :default "NewEnumerator8"))
  (if (and (Variables|State|GetIsActive) (Utilities|Enum|Equal(Enum) Interaction "NewEnumerator6"))
    (Variables|/Game/Blueprints/Player/BP_CorgiCharacter.BP_CorgiCharacter_C|SetItemGrabbed PlayerCharacter self) ; Reference ourselves in.
    (Physics|SetSimulatePhysics (Variables|Default|GetItemMesh) false) ; Turn off item mesh physics.
    (Collision|SetCollisionEnabled (Variables|Default|GetItemMesh) "NoCollision") ; Turn off item mesh collision.
    (Transformation|AttachActorToActor PlayerCharacter "None" "KeepWorld" "KeepRelative" "KeepRelative" false) ; Attach ourselves to the player.
    (Development|PrintString "Hello")))

(fn ConstructionScript)