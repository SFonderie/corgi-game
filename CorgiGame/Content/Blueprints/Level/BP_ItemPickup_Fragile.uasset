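; Fragile item pickup that breaks if the corgi player character carries it too fast for too long.
; Each Tick with a valid carrier, it compares the character's squared last-update velocity to squared MaxSpeed, adding frame time to Damage while over the limit.
; Damage never recovers here; once it reaches Durability, the item clears the character's ItemGrabbed reference, destroys itself and prints a debug message.
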(event EventTick
  (params (DeltaSeconds :type Float%20%28single-precision%29))
  (bind _carrying_actor (CallFunction|GetCarrier))
  (Utilities|IsValid _carrying_actor ; Only update if the carrier is valid.
    (:Is%20Valid
      (bind _asbp_corgi_character (Utilities|Casting|CastToBP_CorgiCharacter _carrying_actor)) ; Only the player character can damage\nthis item.
      (bind _output_get (Variables|State|SetDamage (+ (Variables|State|GetDamage) (Math|Float|SelectFloat DeltaSeconds 0.0 (> (Math|Vector|VectorLengthSquared (Pawn|Components|CharacterMovement|GetLastUpdateVelocity (Variables|/Script/Engine.Character|GetCharacterMovement _asbp_corgi_character))) (Math|Float|Square (Variables|Settings|GetMax%20Speed))))))) ; New damage value\nfor this tick.
      (if (>= _output_get (Variables|Settings|GetDurability)) ; If we take enough damage...
        (Variables|/Game/Blueprints/Player/BP_CorgiCharacter.BP_CorgiCharacter_C|SetItemGrabbed _asbp_corgi_character 0) ; Clear the player's reference\nso that they also know that\nwe are destroyed...
        (Actor|DestroyActor) ; Then boom. Gone.
        (Development|PrintString "DEATH")))))

(fn ConstructionScript
  (|CallParentFunction))