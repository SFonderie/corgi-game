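; BP_EventSequencer is a level trigger that turns a player interaction into an ordered sequence of notifications to listeners.
; OnInteraction proceeds only if the interaction matches the mask and every InteractionChecks entry validates the player.
; Each Sequence step has a pre-delay ahead of its OnSequence calls to that step's listeners.
; ForceSequence bypasses both checks and runs the same sequence with the player's BP_CorgiCharacter.
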(event Custom|Force%20Sequence
  (bind _asbp_corgi_character (Utilities|Casting|CastToBP_CorgiCharacter (Game|GetPlayerCharacter 0)))
  (for _array_element (Variables|Sequence|GetSequence) ; Now we can finally execute\nthe sequence.
    (Utilities|FlowControl|Delay (.PreDelay (Utilities|Struct|BreakBPS_SequencerPhase _array_element))) ; Wait for the pre-delay...
    (for _array_element_2 (.Listener (Utilities|Struct|BreakBPS_SequencerPhase _array_element)) ; At last, notify each listener.
      (Default|OnSequence _array_element_2 self _asbp_corgi_character))))

(event EventOnInteraction
  (params (PlayerCharacter :type BP%20Corgi%20Character%20Object%20Reference) (Interaction :type BPE_Interaction%20Enum :default "NewEnumerator8"))
  (if (CallFunction|CheckInteractionMask (Variables|Sequence|GetInteractionMask) Interaction) ; Only allow interactions\nthat match the mask.
    (if (CallFunction|CheckEvent PlayerCharacter) ; Only continue if all of the\nchecks pass.
      (for _array_element (Variables|Sequence|GetSequence) ; Now we can finally execute\nthe sequence.
        (Utilities|FlowControl|Delay (.PreDelay (Utilities|Struct|BreakBPS_SequencerPhase _array_element))) ; Wait for the pre-delay...
        (for _array_element_2 (.Listener (Utilities|Struct|BreakBPS_SequencerPhase _array_element)) ; At last, notify each listener.
          (Default|OnSequence _array_element_2 self PlayerCharacter))))))

(fn ConstructionScript)

(fn CheckEvent
  (params (Invoker :type BP%20Corgi%20Character%20Object%20Reference))
  (LocalVariables|SetIsValidOverall true) ; Local flag starts true and will\nbe tripped by a single false.
  (for _array_element (Variables|Sequence|GetInteractionChecks) ; Iterate through the checks.\nIf even one returns false,\nthen return invalid.
    (bind _isvalid (Default|ValidateInteraction _array_element Invoker)) ; Check the invoker to validate\nthe interaction.
    (LocalVariables|SetIsValidOverall (and _isvalid (LocalVariables|GetIsValidOverall))))
  (return (LocalVariables|GetIsValidOverall)))