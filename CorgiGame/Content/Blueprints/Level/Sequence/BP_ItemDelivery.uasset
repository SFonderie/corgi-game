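; Level sequence Blueprint that handles delivery of a specific item by the player.
; Interaction is valid only when the invoker's grabbed item is the configured DeliverActor.
; When the sequence fires, it calls OnPlayerDeliver on that item with the player, target and socket.
; Without a valid DeliverTarget, it destroys the item instead.
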(event EventOnSequence
  (params (Event%20Sequencer :type BP%20Event%20Sequencer%20Object%20Reference) (Player%20Character :type BP%20Corgi%20Character%20Object%20Reference))
  (bind _delivertarget (Variables|Sequence|GetDeliverTarget))
  (Utilities|IsValid _delivertarget ; Deliver if there is a delivery target;\ndelete if there is no target.
    (:Is%20Valid
      (Default|OnPlayerDeliver (Variables|Check|GetDeliverActor) Player%20Character _delivertarget (Variables|Sequence|GetDeliverSocket)))
    (:Is%20Not%20Valid
      (Actor|DestroyActor (Variables|Check|GetDeliverActor)))))

(fn ConstructionScript)

(fn ValidateInteraction
  (params (Invoker :type BP%20Corgi%20Character%20Object%20Reference))
  (return (== (Variables|/Game/Blueprints/Player/BP_CorgiCharacter.BP_CorgiCharacter_C|GetItemGrabbed Invoker) (Variables|Check|GetDeliverActor))))