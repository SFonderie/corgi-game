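; BP_EventTrigger is a level trigger actor that relays overlap and player interaction events to a list of listeners.
; Begin and end overlaps are filtered to Character actors, then forwarded to each entry in EventListeners as OnTriggerEnter or OnTriggerExit.
; OnPlayerInteract passes the player character and interaction to every listener's OnInteraction, decoupling the trigger from the objects that respond.
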(event EventOnPlayerInteract
  (params (PlayerCharacter :type BP%20Corgi%20Character%20Object%20Reference) (Interaction :type BPE_Interaction%20Enum :default "NewEnumerator8"))
  (for _array_element (Variables|Trigger|GetEventListeners) ; Loop through the listeners.
    (Default|OnInteraction _array_element PlayerCharacter Interaction)))

(event Collision|EventActorBeginOverlap
  (params (OtherActor :type Actor%20Object%20Reference))
  (bind _ascharacter (Utilities|Casting|CastToCharacter OtherActor)) ; Only deploy if the actor is a\ncharacter pawn.
  (for _array_element (Variables|Trigger|GetEventListeners) ; Loop through the listeners.
    (Default|OnTriggerEnter _array_element _ascharacter)))

(event Collision|EventActorEndOverlap
  (params (OtherActor :type Actor%20Object%20Reference))
  (bind _ascharacter (Utilities|Casting|CastToCharacter OtherActor)) ; Only deploy if the actor is a\ncharacter pawn.
  (for _array_element (Variables|Trigger|GetEventListeners) ; Loop through the listeners.
    (Default|OnTriggerExit _array_element _ascharacter)))

(fn ConstructionScript)