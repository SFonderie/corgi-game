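; Paired level trigger that teleports the player between itself and its Mirror trigger on a specific interaction.
; On BeginPlay it sets itself as the Mirror's partner if that has none, so one-way links become two-way.
; Interaction plays the LS_FlipFade sequence, then moves the player after a fixed delay, preserving their offset from the trigger.
; A CanTeleport flag blocks repeat presses until a second delay ends and the sequence actor is destroyed.
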(event EventOnInteraction
  (params (PlayerCharacter :type BP%20Corgi%20Character%20Object%20Reference) (Interaction :type BPE_Interaction%20Enum :default "NewEnumerator8"))
  (if (Utilities|Enum|Equal(Enum) Interaction "NewEnumerator4")
    (if (Variables|Default|GetCanTeleport) ; Ensure that button spam\ncannot break the flip.
      (Variables|Default|SetCanTeleport false)
      (bind (_outactor _returnvalue) (Sequencer|Player|CreateLevelSequencePlayer "/Game/Blueprints/Function/LS_FlipFade.LS_FlipFade")) ; Create a new level sequence player for the\nfade sequence and plop it... somewhere.
      (Sequencer|Player|Play _returnvalue :!class /Script/MovieScene.MovieSceneSequencePlayer) ; Actually play the level sequence.
      (Utilities|FlowControl|Delay 1.0) ; Hard-coded delay.
      (Transformation|Teleport PlayerCharacter
        (:next
          (Utilities|FlowControl|Delay 1.0) ; Hard-coded delay.
          (Actor|DestroyActor _outactor)
          (Variables|Default|SetCanTeleport true))))))

(event EventBeginPlay
  (Utilities|IsValid (Variables|Default|GetMirror)
    (:Is%20Valid
      (Utilities|IsValid (Variables|BP_FlipFlopTrigger_C|GetMirror (Variables|Default|GetMirror)) ; If we're connected to something\nand it's not connected to anything,\nconnect it to ourselves.
        (:Is%20Not%20Valid
          (Variables|BP_FlipFlopTrigger_C|SetMirror (Variables|Default|GetMirror) self))))))

(fn ConstructionScript)