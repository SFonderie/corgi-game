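; BP_ItemRespawner is a level actor that respawns a fragile item pickup whenever it is destroyed.
; On BeginPlay it records the RespawnTarget's transform, Durability and MaxSpeed, then binds to its OnDestroyed event.
; When that pickup is destroyed, it spawns a new BP_ItemPickup_Fragile at the saved transform, copies the saved values and rebinds, so respawning repeats indefinitely.
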(event Custom|On%20Target%20Destroyed
  (params (DestroyedActor :type Actor%20Object%20Reference))
  ;[1 1 1] This would work infinitely better in C++ for an extremely dumb reason
  (bind _asbp_item_pickup_fragile (Utilities|Casting|CastToBP_ItemPickup_Fragile DestroyedActor)) ; Check to see if the actor is the right type.
  (if (== _asbp_item_pickup_fragile (Variables|State|GetCurrentTarget)) ; Verify we have the right\nactor.
    (bind _returnvalue (Game|SpawnActorfromClass "/Game/Blueprints/Level/BP_ItemPickup_Fragile.BP_ItemPickup_Fragile_C" (Variables|State|GetSpawnPoint) "AdjustIfPossibleButAlwaysSpawn" 0 0)) ; Create the new actor and spawn it at our tracked point.
    (Variables|State|SetCurrentTarget _returnvalue) ; Replace our reference.
    (Variables|/Game/Blueprints/Level/BP_ItemPickup_Fragile.BP_ItemPickup_Fragile_C|SetDurability _returnvalue (Variables|State|GetDurabilityValue)) ; Copy durability.
    (Variables|/Game/Blueprints/Level/BP_ItemPickup_Fragile.BP_ItemPickup_Fragile_C|SetMax%20Speed _returnvalue (Variables|State|GetMaxSpeedValue)) ; Copy max speed.
    (Game|BindEventtoOnDestroyed _returnvalue (delegate Custom|On%20Target%20Destroyed)) ; Allows us to react when the actor\nis destroyed.
  ))

(event EventBeginPlay
  ;[1 1 1] This would work infinitely better in C++ for an extremely dumb reason
  (bind _output_get (Variables|State|SetCurrentTarget (Variables|Settings|GetRespawnTarget)))
  (Variables|State|SetSpawnPoint (Transformation|GetActorTransform _output_get))
  (Variables|State|SetDurabilityValue (Variables|/Game/Blueprints/Level/BP_ItemPickup_Fragile.BP_ItemPickup_Fragile_C|GetDurability _output_get))
  (Variables|State|SetMaxSpeedValue (Variables|/Game/Blueprints/Level/BP_ItemPickup_Fragile.BP_ItemPickup_Fragile_C|GetMax%20Speed _output_get))
  (Game|AssignOnDestroyed _output_get (delegate Custom|On%20Target%20Destroyed)) ; Allows us to react when the actor\nis destroyed.
)

(fn ConstructionScript)